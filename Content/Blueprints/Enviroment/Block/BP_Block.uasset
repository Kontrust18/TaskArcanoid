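; BP_Block is a destructible block that awards a point to the player whose projectile hits it.
; On BeginPlay it creates a dynamic material instance on its mesh and sets the color to either a random darker tint or ColorBlock, depending on RandomColor.
; BlockHit finds the projectile's instigating BP_PlayerController, increments its Points, destroys the block and returns true.
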(event `self.ReceiveBeginPlay`
  (`self.SetColorBlock`))

(fn `BlockHit`
  (params (Projectile :type "/Game/Blueprints/Projectiles/BP_Projectile Object Reference"))
  (returns (Success :type Boolean))
  (bind _asbp_player_controller (cast `/Game/Blueprints/Gamemode/BP_PlayerController` (`self.GetInstigatorController` Projectile)))
  (`/Engine/EditorBlueprintResources/StandardMacros.IncrementInt` (`/Game/Blueprints/Gamemode/BP_PlayerController.Points` _asbp_player_controller)
    (:`  `
      (`self.K2_DestroyActor`)
      (return true))))

(fn `SetColorBlock`
  (bind _returnvalue (`PrimitiveComponent.CreateDynamicMaterialInstance` (`self.Mesh`) 0 "/Game/Assets/Materials/Block/M_Block_Inst.M_Block_Inst" "Color"))
  (`MaterialInstanceDynamic.SetVectorParameterValue` _returnvalue "Color" (select `bool` (`self.RandomColor`) :`false` (`self.ColorBlock`) :`true` (make `LinearColor` (`KismetMathLibrary.RandomFloatInRange` 0.0 0.5) (`KismetMathLibrary.RandomFloatInRange` 0.0 0.5) (`KismetMathLibrary.RandomFloatInRange` 0.0 0.5) (`KismetMathLibrary.RandomFloatInRange` 0.0 0.2)))))

(fn `UserConstructionScript`)