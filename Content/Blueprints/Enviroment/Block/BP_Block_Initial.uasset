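; Destructible block that seeds a row of further blocks along world Y at BeginPlay on the server.
; Each step sphere-traces for free space, then on a coin flip spawns a class picked by ordered chance rolls over BlockInfos, falling back to the last entry.
; A dynamic material instance tints it randomly or with ColorBlock.
; BlockHit gives the projectile's instigating player controller a point and destroys the block.
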(event `self.ReceiveBeginPlay`
  (`self.SetColorBlock`)
  (if (`KismetSystemLibrary.IsServer`)
    (`self.StartGenerateLinear`)))

(fn `BlockHit`
  (params (Projectile :type "/Game/Blueprints/Projectiles/BP_Projectile Object Reference"))
  (returns (Success :type Boolean))
  (bind _asbp_player_controller (cast `/Game/Blueprints/Gamemode/BP_PlayerController` (`self.GetInstigatorController` Projectile))
    (:`then`
      (`/Engine/EditorBlueprintResources/StandardMacros.IncrementInt` (`/Game/Blueprints/Gamemode/BP_PlayerController.Points` _asbp_player_controller)
        (:`  `
          (`self.K2_DestroyActor`)
          (return true))))
    (:`CastFailed`
      (return false))))

(fn `CheckClass`
  (returns (Class :type "/Game/Blueprints/Enviroment/Block/BP_Block Class Reference"))
  (locals (L_Class :type "/Game/Blueprints/Enviroment/Block/BP_Block Class Reference"))
  (for _array_element (`self.BlockInfos`)
    (bind (_blockclass _chance) (break `/Game/Data/Structures/ST_BlockInfo` _array_element))
    (set `local.L_Class` _blockclass)
    (if (>= _chance (`KismetMathLibrary.RandomFloatInRange` 0.0 100.0))
      (break)))
  (return (`local.L_Class`)))

(fn `LineTrace`
  (params (Start :type "Vector Structure") (End :type "Vector Structure"))
  (returns (ReturnValue :type Boolean) (TraceEnd :type "Vector Structure"))
  (bind _returnvalue (+ Start (0.0 0.0 20.0)))
  (bind (_outhit _returnvalue_2) (`KismetSystemLibrary.SphereTraceSingleForObjects` _returnvalue (+ _returnvalue End) 20.0 (`|MakeArray` "ObjectTypeQuery1" "ObjectTypeQuery3" "ObjectTypeQuery4" "ObjectTypeQuery7" :!type "EObjectTypeQuery Enum")))
  (return _returnvalue_2 (`.TraceEnd` (`GameplayStatics.BreakHitResult` _outhit))))

(fn `SetColorBlock`
  (bind _returnvalue (`PrimitiveComponent.CreateDynamicMaterialInstance` (`self.Mesh`) 0 "/Game/Assets/Materials/Block/M_Block_Inst.M_Block_Inst" "Color"))
  (`MaterialInstanceDynamic.SetVectorParameterValue` _returnvalue "Color" (select `bool` (`self.RandomColor`) :`false` (`self.ColorBlock`) :`true` (make `LinearColor` (`KismetMathLibrary.RandomFloatInRange` 0.0 0.5) (`KismetMathLibrary.RandomFloatInRange` 0.0 0.5) (`KismetMathLibrary.RandomFloatInRange` 0.0 0.5) (`KismetMathLibrary.RandomFloatInRange` 0.0 0.2)))))

(fn `StartGenerateLinear`
  (for _index (range 12)
    (bind (_returnvalue _traceend) (`self.LineTrace` (+ (`KismetMathLibrary.MakeVector` 0.0 (* _index 110.0)) (`self.K2_GetActorLocation`)) (0.0 120.0 0.0)))
    (if (and (not _returnvalue) (select `bool` (<= (`KismetMathLibrary.RandomFloatInRange` 0.0 100.0) 50.0) :`true` true))
      (`|SpawnActorFromClass` (`self.CheckClass`) (`KismetMathLibrary.MakeTransform` (- _traceend (0.0 20.0 20.0))) "AlwaysSpawn" "OverrideRootScale" null (`self.Gamemode`) null))))

(fn `UserConstructionScript`)