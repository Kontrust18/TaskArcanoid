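; BP_Block_Bonus_Double is a bonus block that duplicates the projectile that hits it.
; On BlockHit it spawns a new BP_Projectile at the hitting projectile's location with yaw offset by 30 degrees, keeping its owner and instigator.
; The new projectile copies the original's speed and color, then the parent block's hit logic runs and its result is returned.
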(fn `BlockHit`
  (params (Projectile :type "/Game/Blueprints/Projectiles/BP_Projectile Object Reference"))
  (returns (Success :type Boolean))
  (locals (L_Projectile :type "/Game/Blueprints/Projectiles/BP_Projectile Object Reference"))
  (bind _l_projectile (`local.L_Projectile`))
  (bind _l_projectile_2 (`local.L_Projectile`))
  (bind _l_projectile_3 (`local.L_Projectile`))
  (bind (_returnvalue_roll _returnvalue_pitch _returnvalue_yaw) (`KismetMathLibrary.BreakRotator` (`self.K2_GetActorRotation` _l_projectile)))
  (set `local.L_Projectile` Projectile)
  (bind _returnvalue (`|SpawnActorFromClass` "/Game/Blueprints/Projectiles/BP_Projectile.BP_Projectile_C" (`KismetMathLibrary.MakeTransform` (`self.K2_GetActorLocation` _l_projectile) (`KismetMathLibrary.MakeRotator` _returnvalue_roll _returnvalue_pitch (+ _returnvalue_yaw 30.0))) "Undefined" "OverrideRootScale" (`self.GetOwner` _l_projectile_2) (`Actor.Instigator` _l_projectile_2)))
  (set `/Game/Blueprints/Projectiles/BP_Projectile.Speed` (`/Game/Blueprints/Projectiles/BP_Projectile.Speed` _l_projectile_3) _returnvalue)
  (set `/Game/Blueprints/Projectiles/BP_Projectile.Color` (`/Game/Blueprints/Projectiles/BP_Projectile.Color` _l_projectile_3) _returnvalue)
  (bind _success (`parent.BlockHit` (`local.L_Projectile`)))
  (return _success))

(fn `UserConstructionScript`
  (`parent.UserConstructionScript`))