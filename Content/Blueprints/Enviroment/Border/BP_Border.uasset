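; BP_Border is an environment border piece with a configurable color that reacts to projectile hits.
; The ColorBorder RepNotify calls SetColorBorder, which creates a dynamic material instance on the mesh and sets its Color parameter.
; HitProjectile passes the hit location to the ClientSpawnParticle and ClientSpawnSound events, which spawn an explosion effect and a laser shot sound there.
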(event `ClientSpawnParticle`
  (params (EmitterTemplate :type "ParticleSystem Object Reference") (Location :type "Vector Structure"))
  (`GameplayStatics.SpawnEmitterAtLocation` EmitterTemplate Location))

(event `ClientSpawnSound`
  (params (Sound :type "SoundBase Object Reference") (Location :type "Vector Structure"))
  (`GameplayStatics.SpawnSoundAtLocation` Sound Location (struct) 1.0 1.0 0.0 null null))

(fn `HitProjectile`
  (params (Location :type "Vector Structure"))
  (locals (L_Location :type "Vector Structure"))
  (set `local.L_Location` Location)
  (`self.ClientSpawnParticle` "/Game/Assets/Particles/P_Explosion2.P_Explosion2" (`local.L_Location`))
  (`self.ClientSpawnSound` "/Game/Assets/Sounds/LaserShot_Cue.LaserShot_Cue" (`local.L_Location`)))

(fn `OnRep_ColorBorder`
  (`self.SetColorBorder`))

(fn `SetColorBorder`
  (bind _returnvalue (`PrimitiveComponent.CreateDynamicMaterialInstance` (`self.Mesh`) 0 "/Game/Assets/Materials/PlayerColors/M_Color_Inst.M_Color_Inst" "Color"))
  (`MaterialInstanceDynamic.SetVectorParameterValue` _returnvalue "Color" (`self.ColorBorder`)))

(fn `UserConstructionScript`)