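; BP_Obstacle is a level obstacle that randomly fills a straight row with copies of itself.
; On BeginPlay, only an instance flagged Initial runs the generation, and only on the server.
; StartGenerateLinear steps along world Y in both directions at fixed spacing, line-tracing each segment and stopping that direction at the first hit.
; Each clear segment has a 30% chance to spawn the same class near the trace end.
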(event `self.ReceiveBeginPlay`
  (if (and (`self.Initial`) (`KismetSystemLibrary.IsServer`))
    (`self.StartGenerateLinear`)))

(fn `LineTrace`
  (params (Start :type "Vector Structure") (End :type "Vector Structure"))
  (returns (ReturnValue :type Boolean) (TraceEnd :type "Vector Structure"))
  (bind _returnvalue (+ Start (0.0 0.0 20.0)))
  (bind (_outhit _returnvalue_2) (`KismetSystemLibrary.LineTraceSingleForObjects` :`Start` _returnvalue :`End` (+ _returnvalue End) :`ObjectTypes` (`|MakeArray` "ObjectTypeQuery1" "ObjectTypeQuery2" "ObjectTypeQuery3" "ObjectTypeQuery4" :!type "EObjectTypeQuery Enum") :`bTraceComplex` true :`DrawTime` 50.0))
  (return _returnvalue_2 (`.TraceEnd` (`GameplayStatics.BreakHitResult` _outhit))))

(fn `StartGenerateLinear`
  (for _index (range 11)
    (bind (_returnvalue _traceend) (`self.LineTrace` (+ (`KismetMathLibrary.MakeVector` 0.0 (* _index 100.0)) (`self.K2_GetActorLocation`)) (0.0 120.0 0.0)))
    (if (not _returnvalue)
      (if (select `bool` (<= (`KismetMathLibrary.RandomFloatInRange` 0.0 100.0) 30.0) :`true` true)
        (`|SpawnActorFromClass` (`GameplayStatics.GetObjectClass` self) (`KismetMathLibrary.MakeTransform` (- _traceend (0.0 20.0 20.0))) "AlwaysSpawn" "OverrideRootScale" null false null))
      (else
        (break))))
  (for _index_2 (range 11)
    (bind (_returnvalue_2 _traceend_2) (`self.LineTrace` (+ (`KismetMathLibrary.MakeVector` 0.0 (* _index_2 -100.0)) (`self.K2_GetActorLocation`)) (0.0 -120.0 0.0)))
    (if (not _returnvalue_2)
      (if (select `bool` (<= (`KismetMathLibrary.RandomFloatInRange` 0.0 100.0) 30.0) :`true` true)
        (`|SpawnActorFromClass` (`GameplayStatics.GetObjectClass` self) (`KismetMathLibrary.MakeTransform` (- _traceend_2 (0.0 -20.0 20.0))) "AlwaysSpawn" "OverrideRootScale" null false null))
      (else
        (break)))))

(fn `UserConstructionScript`)