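; Server game mode for a two-player Arkanoid-style level that registers and spawns both players, generates the board and runs the round end.
; On BeginPlay the authority spawns random obstacles and a row of initial blocks.
; When no blocks remain or both players are out, it destroys projectiles and collects each player's points.
; Scores go to client end menus, and two OK confirmations advance the GameInstance to the next level.
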(event `ServerChekBlocks`
  ;[0.225 0.2393 1] CheckBlocks
  (`self.CheckBlocks`))

(event `self.ReceiveBeginPlay`
  ;[0.11 1 0.3157] BeginPlay and StartGenerate
  (`/Engine/EditorBlueprintResources/ActorMacros.Switch Has Authority`
    (:`Authority`
      (`self.StartGenerateObstacles`))))

(event `ServerChekGameOverPlayers`
  ;[0.5708 0 0] CheckGameOverPlayers
  (bind _result (`/Engine/EditorBlueprintResources/StandardMacros.IncrementInt` (`self.GameOverPlayers`))
    (:`  `
      (if (>= _result 2)
        (`|ExecutionSequence`
          (:`then_0`
            (bind _outactors (`GameplayStatics.GetAllActorsOfClass` "/Game/Blueprints/Projectiles/BP_Projectile.BP_Projectile_C"))
            (for _array_element _outactors
              (`/Game/Blueprints/Projectiles/BP_Projectile.MultiDestoy` _array_element)))
          (:`then_1`
            (for _array_element_2 (`self.Players`)
              (`/Game/Blueprints/Gamemode/BP_PlayerController.ClientPointsToServer` _array_element_2))))))))

(event `ServerSetPoints`
  (params (Index :type Integer) (Server :type Integer))
  ;[0.6833 0.5266 0] EndGame
  (if (< Index 1)
    (set `self.PointsPlayer01` Server)
    (else
      (set `self.PointsPlayer02` Server)))
  (for _array_element (`self.Players`)
    (`/Game/Blueprints/Gamemode/BP_PlayerController.ClientCreateEndMenu` _array_element (`self.PointsPlayer01`) (`self.PointsPlayer02`))))

(event `ServerCheckOk`
  ;[0.6833 0.5266 0] EndGame
  (bind _result (`/Engine/EditorBlueprintResources/StandardMacros.IncrementInt` (`self.PressedOk`))
    (:`  `
      (if (>= _result 2)
        (bind _asbp_game_instance (cast `/Game/Blueprints/Gamemode/BP_GameInstance` (`GameplayStatics.GetGameInstance`)))
        (`/Game/Blueprints/Gamemode/BP_GameInstance.NextLevel` _asbp_game_instance)))))

(fn `CheckBlocks`
  (locals (L_Check :type Boolean))
  (bind _outactors (`GameplayStatics.GetAllActorsOfClass` "/Game/Blueprints/Enviroment/Block/BP_Block.BP_Block_C"))
  (if (not (`KismetSystemLibrary.IsValid` (`|GetArrayItem` _outactors)))
    (bind _outactors_2 (`GameplayStatics.GetAllActorsOfClass` "/Game/Blueprints/Enviroment/Block/BP_Block_Initial.BP_Block_Initial_C"))
    (if (not (`KismetSystemLibrary.IsValid` (`|GetArrayItem` _outactors_2)))
      (`|ExecutionSequence`
        (:`then_0`
          (bind _outactors_3 (`GameplayStatics.GetAllActorsOfClass` "/Game/Blueprints/Projectiles/BP_Projectile.BP_Projectile_C"))
          (for _array_element _outactors_3
            (`/Game/Blueprints/Projectiles/BP_Projectile.MultiDestoy` _array_element)))
        (:`then_1`
          (for _array_element_2 (`self.Players`)
            (`/Game/Blueprints/Gamemode/BP_PlayerController.ClientPointsToServer` _array_element_2)))))))

(fn `ChoosePlayerStart`
  (params (Player :type "Controller Object Reference"))
  (returns (ReturnValue :type "Actor Object Reference"))
  (locals (L_Player :type "/Game/Blueprints/Gamemode/BP_PlayerController Object Reference"))
  (bind _asbp_player_controller (cast `/Game/Blueprints/Gamemode/BP_PlayerController` Player))
  (bind _output_get (set `local.L_Player` _asbp_player_controller))
  (bind _returnvalue (`KismetArrayLibrary.Array_Add` (`self.Players`) _output_get))
  (set `/Game/Blueprints/Gamemode/BP_PlayerController.Index` _returnvalue (`local.L_Player`))
  (set `/Game/Blueprints/Gamemode/BP_PlayerController.Gamemode` self (`local.L_Player`))
  (bind _outactors (`GameplayStatics.GetAllActorsOfClass` "/Script/Engine.PlayerStart"))
  (return (`|GetArrayItem` _outactors (`/Game/Blueprints/Gamemode/BP_PlayerController.Index` (`local.L_Player`)))))

(fn `StartGenerateBlocks`
  (if (`KismetSystemLibrary.IsServer`)
    (for _index (range 11)
      (`|SpawnActorFromClass` "/Game/Blueprints/Enviroment/Block/BP_Block_Initial.BP_Block_Initial_C" (`KismetMathLibrary.MakeTransform` (`KismetMathLibrary.MakeVector` (`KismetMathLibrary.Conv_IntToDouble` (+ (+ (* _index 70) 70) -355)) -650.0 40.0)) "AdjustIfPossibleButDontSpawnIfColliding" "OverrideRootScale" null self null))))

(fn `StartGenerateObstacles`
  (for _ (range (+ (`KismetMathLibrary.RandomIntegerInRange` 0 6) 1))
    (`|SpawnActorFromClass` "/Game/Blueprints/Enviroment/Obstacle/BP_Obstacle.BP_Obstacle_C" (`KismetMathLibrary.MakeTransform` (`KismetMathLibrary.MakeVector` (`KismetMathLibrary.Conv_IntToDouble` (* (`KismetMathLibrary.RandomIntegerInRange` -6 6) 50)) (`KismetMathLibrary.Conv_IntToDouble` (* (`KismetMathLibrary.RandomIntegerInRange` -6 6) 100)))) "AlwaysSpawn" "OverrideRootScale" null true null))
  (`self.StartGenerateBlocks`))

(fn `UserConstructionScript`)