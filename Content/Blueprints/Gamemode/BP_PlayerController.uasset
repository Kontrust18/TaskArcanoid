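; Player controller for a networked game with two-player results, managing each client's HUD, game over state and end menu.
; RepNotifies update health and points on the HUD; at zero health the client shows game over and calls the server to remove the pawn and notify the game mode.
; Client and server events relay points and OK confirmations to the game mode and display both players' results.
; Player index selects a red or blue color.
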(event `self.ReceiveBeginPlay`
  ;[0.1625 0.1787 1] BeginPlay and Create HUD
  (`/Engine/EditorBlueprintResources/ActorMacros.Switch Has Authority`
    (:`Remote`
      (`self.CreateHUD`))))

(event `ServerGameOver`
  ;[1 0.1665 0.1824] GameOver
  (set `self.GameOver` true)
  (bind _asbp_player_pawn (cast `/Game/Blueprints/Pawns/BP_PlayerPawn` (`self.K2_GetPawn`)))
  (`/Game/Blueprints/Pawns/BP_PlayerPawn.ServerRemovePawn` _asbp_player_pawn)
  (`/Game/Blueprints/Gamemode/BP_ArcanoidGamemode.ServerChekGameOverPlayers` (`self.Gamemode`)))

(event `ClientPointsToServer`
  ;[1 0.6876 0.1566] EndGame
  (`self.ServerSendPointsToGamemode` (`self.Index`) (`self.Points`)))

(event `ServerSendOk`
  ;[0.3009 1 0.2433] SendOk
  (`/Game/Blueprints/Gamemode/BP_ArcanoidGamemode.ServerCheckOk` (`self.Gamemode`)))

(event `ServerSendPointsToGamemode`
  (params (Index :type Integer) (Server :type Integer))
  ;[1 0.6876 0.1566] EndGame
  (`/Game/Blueprints/Gamemode/BP_ArcanoidGamemode.ServerSetPoints` (`self.Gamemode`) Index Server))

(event `ClientCreateEndMenu`
  (params (Player01 :type Integer) (Player02 :type Integer))
  ;[1 0.6876 0.1566] EndGame
  (bind _w_endmenu (`self.W_EndMenu`)
    (:`then`
      (set `/Game/UI/EndMenu/W_EndMenu.Player01` Player01 _w_endmenu)
      (set `/Game/UI/EndMenu/W_EndMenu.Player02` Player02 _w_endmenu))
    (:`else`
      (`self.CreateEndMenu` Player01 Player02))))

(fn `CreateEndMenu`
  (params (Player01 :type Integer) (Player02 :type Integer))
  (bind _returnvalue (`|CreateWidget` "/Game/UI/EndMenu/W_EndMenu.W_EndMenu_C" self Player01 Player02 self))
  (set `self.W_EndMenu` _returnvalue)
  (`Widget.RemoveFromParent` (`self.W_HUD`))
  (`UserWidget.AddToViewport` (`self.W_EndMenu`) 0)
  (set `self.bShowMouseCursor` true)
  (`WidgetBlueprintLibrary.SetInputMode_GameAndUIEx` self (`self.W_EndMenu`) "DoNotLock" false))

(fn `CreateHUD`
  (bind _returnvalue (`|CreateWidget` "/Game/UI/HUD/W_HUD.W_HUD_C" self self))
  (bind _output_get (set `self.W_HUD` _returnvalue))
  (`UserWidget.AddToViewport` _output_get 0)
  (set `self.bShowMouseCursor` false)
  (`WidgetBlueprintLibrary.SetInputMode_GameOnly` self))

(fn `OnRep_GameOver`)

(fn `OnRep_Health`
  (if (not (`KismetSystemLibrary.IsServer`))
    (if (<= (`self.Health`) 0)
      (bind _w_hud (`self.W_HUD`)
        (:`then`
          (`/Game/UI/HUD/W_HUD.SetGameOver` _w_hud)
          (`self.ServerGameOver`))
        (:`else`))
      (else
        (bind _w_hud_2 (`self.W_HUD`)
          (:`then`
            (`/Game/UI/HUD/W_HUD.SetHealth` _w_hud_2))
          (:`else`))))))

(fn `OnRep_Points`
  (if (not (`KismetSystemLibrary.IsServer`))
    (bind _w_hud (`self.W_HUD`)
      (:`then`
        (`/Game/UI/HUD/W_HUD.SetPoints` _w_hud))
      (:`else`))))

(fn `SetColorController`
  (if (> (`self.Index`) 0)
    (set `self.Color` (struct :`G` 0.003008 :`B` 0.633333 :`A` 1.0))
    (else
      (set `self.Color` (struct :`R` 1.0 :`A` 1.0)))))

(fn `UserConstructionScript`)