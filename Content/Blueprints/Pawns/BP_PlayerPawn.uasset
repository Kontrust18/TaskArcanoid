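; Networked player pawn that slides sideways within a limit and launches a projectile on left click via server events.
; On possession it takes the controller's color, spawns an attached projectile, and back-traces for its BP_Border to color and own it.
; Damage costs controller health and starts a recovery timer that respawns the projectile and re-enables launching.
; ServerRemovePawn plays explosion effects and destroys the pawn's components, while OnRep_ColorPawn applies the color through a dynamic material.
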(event Custom|ServerMove
  (params (Axis :type Float%20%28double-precision%29))
  ;[0 0.525 0.07287] Move
  (CallFunction|Move Axis))

(event Custom|ServerStart
  ;[0 0.525 0.07287] Start
  (Transformation|DetachFromActor (Variables|Default|GetProjectile) "KeepWorld" "KeepWorld" "KeepRelative")
  (Variables|/Game/Blueprints/Projectiles/BP_Projectile.BP_Projectile_C|SetSpeed (Variables|Default|GetProjectile) 5e+02))

(event Custom|ClientSetStarted
  ;[0 0.525 0.07287] Start
  (Variables|Default|SetStarted false))

(event Custom|ServerRemovePawn
  ;[0.5375 0.02209 0] GameOver
  (CallFunction|RemovePawn))

(event Custom|ClientSpawnParticle
  (params (EmitterTemplate :type Particle%20System%20Object%20Reference) (Location :type Vector))
  ;[1 0.9711 0.1352] SpawnParticle
  (Effects|SpawnEmitteratLocation EmitterTemplate Location))

(event Custom|ClientSpawnSound
  (params (Sound :type Sound%20Base%20Object%20Reference) (Location :type Vector))
  ;[1 0.9711 0.1352] SpawnSound
  (Audio|SpawnSoundatLocation Sound Location "0, 0, 0" 1.0 1.0 0.0 0 0))

(event Game|Damage|EventAnyDamage
  (params (Damage :type Float%20%28single-precision%29) (DamageType :type Damage%20Type%20Object%20Reference) (InstigatedBy :type Controller%20Object%20Reference) (DamageCauser :type Actor%20Object%20Reference))
  ;[1 0.01959 0] Damage
  (if (not (Variables|Default|GetRecover))
    (CallFunction|Damaged)))

(event EventPossessed
  (params (NewController :type Controller%20Object%20Reference))
  ;[0.06838 0.1007 0.4208] Possesed
  (bind _asbp_player_controller (Utilities|Casting|CastToBP_PlayerController NewController))
  (Variables|Default|SetPlayer%20Controller _asbp_player_controller)
  (Default|SetColorController (Variables|Default|GetPlayer%20Controller))
  (Variables|Default|SetColorPawn (Variables|/Game/Blueprints/Gamemode/BP_PlayerController.BP_PlayerController_C|GetColor (Variables|Default|GetPlayer%20Controller)))
  (CallFunction|SpawnProjectile)
  (CallFunction|SetBorder))

(event EventTick
  (params (DeltaSeconds :type Float%20%28single-precision%29))
  ;[0 0.525 0.07287] Move
  (Variables|Default|GetCollision
    (:then
      (CallFunction|ServerMove (Class|Actor|GetInputAxisKeyValue)))
    (:else)))

(event Input|MouseEvents|LeftMouseButton
  (params (Key :type Key%20Structure :default "None"))
  ;[0 0.525 0.07287] Start
  (:Pressed
    (if (not (Variables|Default|GetStarted))
      (Variables|Default|SetStarted true)
      (CallFunction|ServerStart))))

(fn ConstructionScript)

(fn Move
  (params (Axis :type Float%20%28double-precision%29))
  (bind _limiter (Variables|Default|GetLimiter))
  (bind _collision (Variables|Default|GetCollision))
  (bind _returnvalue (Transformation|GetWorldLocation _collision))
  (LocalVariables|SetL_Axis Axis)
  (bind _collision_2 (Variables|Default|GetCollision)
    (:then
      (Transformation|AddLocalOffset _collision_2 (Math|Vector|MakeVector 0.0 (|({9B755C95-4941-4409-F966-88B837261AD9}*{A4072E0B-418A-D437-0CE7-E1A07D5A23BB})) 0.0) false false)
      ;[1 1 1] In Limiter
      (bind _collision_3 (Variables|Default|GetCollision)
        (:then
          (Transformation|SetWorldLocation _collision_3 (Math|Vector|MakeVector (.x _returnvalue) (Math|Float|Clamp(Float) (.y _returnvalue) (* _limiter -1.0) _limiter) (.z _returnvalue)) false false))
        (:else)))
    (:else)))

(fn SpawnProjectile
  (bind _projectilestart (Variables|Default|GetProjectileStart)
    (:then
      (bind _returnvalue (Game|SpawnActorfromClass "/Game/Blueprints/Projectiles/BP_Projectile.BP_Projectile_C" (Transformation|GetWorldTransform _projectilestart) "AlwaysSpawn" (Pawn|GetController) self))
      (bind _output_get (Variables|Default|SetProjectile _returnvalue))
      (Transformation|AttachComponentToComponent _output_get (Variables|Default|GetProjectileStart) "None" "SnapToTarget" "SnapToTarget" "KeepRelative" true)
      (Variables|/Game/Blueprints/Projectiles/BP_Projectile.BP_Projectile_C|SetColor (Variables|Default|GetProjectile) (Variables|/Game/Blueprints/Gamemode/BP_PlayerController.BP_PlayerController_C|GetColor (Variables|Default|GetPlayer%20Controller))))
    (:else)))

(fn RotateProjectile
  (params (Axis :type Float%20%28double-precision%29))
  (LocalVariables|SetL_Axis Axis)
  (Transformation|SetRelativeRotation (Variables|Default|GetProjectileStart) (Math|Rotator|MakeRotator 0.0 0.0 (select (!= Axis 0.0) (* (LocalVariables|GetL_Axis) 2e+01) (Math|Random|RandomFloatinRange -2.0 2.0))) false false)
  (Transformation|SetActorRotation (Variables|Default|GetProjectile) (Transformation|GetWorldRotation (Variables|Default|GetProjectileStart))))

(fn SetColorPawn
  (bind _returnvalue (Rendering|Material|CreateDynamicMaterialInstance (Variables|Default|GetMesh) 0 "/Game/Assets/Materials/PlayerColors/M_Color_Inst.M_Color_Inst" "Color" :!class /Script/Engine.PrimitiveComponent))
  (bind _output_get (Variables|Default|SetM_Mesh _returnvalue))
  (Rendering|Material|SetVectorParameterValue _output_get "Color" (Variables|Default|GetColorPawn) :!class /Script/Engine.MaterialInstanceDynamic))

(fn OnRepColorPawn
  (CallFunction|SetColorPawn))

(fn SetBorder
  (bind _collision (Variables|Default|GetCollision))
  (bind _returnvalue (Transformation|GetWorldLocation _collision))
  (bind _outhit (Collision|LineTraceByChannel _returnvalue (- _returnvalue (* (Transformation|GetActorForwardVector) 5e+02)) "TraceTypeQuery1" false 0 "None"))
  (bind _asbp_border (Utilities|Casting|CastToBP_Border (.HitActor (Collision|BreakHitResult _outhit))))
  (LocalVariables|SetL_Border _asbp_border)
  (Variables|/Game/Blueprints/Enviroment/Border/BP_Border.BP_Border_C|SetColorBorder (LocalVariables|GetL_Border) (Variables|Default|GetColorPawn))
  (Actor|SetOwner (LocalVariables|GetL_Border) (Variables|Default|GetPlayer%20Controller)))

(fn Damaged
  (bind _player_controller (Variables|Default|GetPlayer%20Controller))
  (if (not (Variables|/Game/Blueprints/Gamemode/BP_PlayerController.BP_PlayerController_C|GetGameOver _player_controller))
    (Math|Integer|DecrementInt (Variables|/Game/Blueprints/Gamemode/BP_PlayerController.BP_PlayerController_C|GetHealth _player_controller)
      (:%20%20
        (Variables|Default|SetRecover true)
        (Utilities|Time|SetTimerbyFunctionName 0 "Recovered" 2.0)))))

(fn Recovered
  (Variables|Default|SetRecover false)
  (if (not (Variables|/Game/Blueprints/Gamemode/BP_PlayerController.BP_PlayerController_C|GetGameOver (Variables|Default|GetPlayer%20Controller)))
    (CallFunction|SpawnProjectile)
    (CallFunction|ClientSetStarted)))

(fn RemovePawn
  (bind _collision (Variables|Default|GetCollision))
  (bind _returnvalue (Transformation|GetWorldLocation _collision))
  (CallFunction|ClientSpawnParticle "/Game/Assets/Particles/P_Explosion.P_Explosion" _returnvalue)
  (CallFunction|ClientSpawnSound "/Game/Assets/Sounds/Bang_Cue.Bang_Cue" _returnvalue)
  (Components|DestroyComponent (Variables|Default|GetSphere1))
  (Components|DestroyComponent (Variables|Default|GetSphere))
  (Components|DestroyComponent (Variables|Default|GetProjectileStart))
  (Components|DestroyComponent (Variables|Default|GetMesh))
  (Components|DestroyComponent (Variables|Default|GetBox3))
  (Components|DestroyComponent (Variables|Default|GetBox2))
  (Components|DestroyComponent (Variables|Default|GetBox1))
  (Components|DestroyComponent (Variables|Default|GetBox))
  (Components|DestroyComponent (Variables|Default|GetCollision)))