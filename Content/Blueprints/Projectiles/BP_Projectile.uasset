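; Replicated Arkanoid ball for multiplayer, with speed, color and Destroyer state applied through OnReps.
; Server-side hits notify blocks and have the game mode check them, or damage an opposing pawn and destroy other owners' balls.
; Hitting its owner's border destroys the ball, damaging the player if it was their last.
; Bonuses step speed within limits; Destroyer mode uses an overlap mesh to destroy obstacles and hit blocks.
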(event `ClientSpawnSound`
  (params (Sound :type "SoundBase Object Reference"))
  ;[1 0.8568 0.292] ClientSpawnSound
  (`GameplayStatics.SpawnSoundAtLocation` Sound (`self.K2_GetActorLocation`) (struct) 1.0 1.0 0.0 null null))

(event `self.Collision.OnComponentHit`
  (params (HitComponent :type "PrimitiveComponent Object Reference") (OtherActor :type "Actor Object Reference") (OtherComp :type "PrimitiveComponent Object Reference") (NormalImpulse :type "Vector Structure") (Hit :type "HitResult Structure (by ref)"))
  ;[0 1 0.004274] HitActor
  (`/Engine/EditorBlueprintResources/ActorMacros.Switch Has Authority`
    (:`Authority`
      (`self.HitActor` OtherActor Hit))))

(event `MultiDestoy`
  ;[1 0.04911 0.03319] DestroyProhectile
  (`self.K2_DestroyActor`))

(event `self.ReceiveBeginPlay`
  ;[0.138 0.1234 1] BeginPlay
  (`self.SetColorProjectile`))

(event `self.MeshOverlap.OnComponentBeginOverlap`
  (params (OverlappedComponent :type "PrimitiveComponent Object Reference") (OtherActor :type "Actor Object Reference") (OtherComp :type "PrimitiveComponent Object Reference") (OtherBodyIndex :type Integer) (bFromSweep :type Boolean) (SweepResult :type "HitResult Structure (by ref)"))
  ;[1 0.2083 0.8104] OverlapForDestroyerFromBonus
  (if (`self.Destroyer`)
    (bind _asbp_obstacle (cast `/Game/Blueprints/Enviroment/Obstacle/BP_Obstacle` OtherActor)
      (:`then`
        (`self.K2_DestroyActor` _asbp_obstacle)
        (`self.ClientSpawnSound` "/Game/Assets/Sounds/Step2_Cue.Step2_Cue" :!label _label))
      (:`CastFailed`
        (bind _success (message `/Game/Blueprints/Libs/Intefaces/BPI_HitBlock.BlockHit` OtherActor self))
        (if _success
          (bind _asbp_arcanoid_gamemode (cast `/Game/Blueprints/Gamemode/BP_ArcanoidGamemode` (`GameplayStatics.GetGameMode`)))
          (`/Game/Blueprints/Gamemode/BP_ArcanoidGamemode.ServerChekBlocks` _asbp_arcanoid_gamemode)
          (goto _label))))))

(fn `BonusSpeed`
  (params (Up :type Boolean))
  (bind _stagespeed (`self.StageSpeed`))
  (if Up
    (bind _result (`/Engine/EditorBlueprintResources/StandardMacros.IncrementInt` _stagespeed)
      (:`  `
        (if (< _result 3)
          (set `self.Speed` (+ (`self.Speed`) 300.0))
          (else
            (set `self.StageSpeed` 2)))))
    (else
      (bind _result_2 (`/Engine/EditorBlueprintResources/StandardMacros.DecrementInt` _stagespeed)
        (:`  `
          (if (> _result_2 -1)
            (set `self.Speed` (- (`self.Speed`) 300.0))
            (else
              (set `self.StageSpeed` 0))))))))

(fn `HitActor`
  (params (Actor :type "Actor Object Reference") (HitResult :type "HitResult Structure"))
  (locals (L_Actor :type "Actor Object Reference") (L_Border :type "/Game/Blueprints/Enviroment/Border/BP_Border Object Reference") (L_Hit :type "HitResult Structure"))
  (set `local.L_Actor` Actor)
  (set `local.L_Hit` HitResult)
  (`|ExecutionSequence`
    (:`then_0`
      (bind _asbp_border (cast `/Game/Blueprints/Enviroment/Border/BP_Border` (`local.L_Actor`))
        (:`then`
          (set `local.L_Border` _asbp_border)
          (if (== (`self.GetOwner`) (`self.GetOwner` (`local.L_Border`)))
            (`self.HitBorder` (`local.L_Border`) (`local.L_Hit`))))
        (:`CastFailed`
          (bind _asbp_player_pawn (cast `/Game/Blueprints/Pawns/BP_PlayerPawn` (`local.L_Actor`))
            (:`then`
              (if (!= (`self.GetOwner`) (`self.GetOwner` _asbp_player_pawn))
                (`GameplayStatics.ApplyDamage` _asbp_player_pawn 0.01)
                (bind _outactors (`GameplayStatics.GetAllActorsOfClass` "BP_Projectile_C"))
                (for _array_element _outactors
                  (if (!= _array_element self)
                    (if (!= (`self.GetOwner` _array_element) (`self.GetOwner`))
                      (`self.MultiDestoy` _array_element))))
                (`self.ClientSpawnSound` "/Game/Assets/Sounds/LaserShot_Cue.LaserShot_Cue")))
            (:`CastFailed`
              (bind _success (message `/Game/Blueprints/Libs/Intefaces/BPI_HitBlock.BlockHit` (`local.L_Actor`) self))
              (if _success
                (bind _asbp_arcanoid_gamemode (cast `/Game/Blueprints/Gamemode/BP_ArcanoidGamemode` (`GameplayStatics.GetGameMode`)))
                (`/Game/Blueprints/Gamemode/BP_ArcanoidGamemode.ServerChekBlocks` _asbp_arcanoid_gamemode)))))))
    (:`then_1`
      (`self.ClientSpawnSound` "/Game/Assets/Sounds/Step2_Cue.Step2_Cue"))))

(fn `HitBorder`
  (params (Border :type "/Game/Blueprints/Enviroment/Border/BP_Border Object Reference") (Hit :type "HitResult Structure"))
  (locals (L_Border :type "/Game/Blueprints/Enviroment/Border/BP_Border Object Reference") (L_Found :type Boolean) (L_Hit :type "HitResult Structure"))
  (set `local.L_Border` Border)
  (set `local.L_Hit` Hit)
  (bind _outactors (`GameplayStatics.GetAllActorsOfClass` "BP_Projectile_C"))
  (for _array_element _outactors
    (if (!= _array_element self)
      (if (== (`self.GetOwner` _array_element) (`self.GetOwner`))
        (set `local.L_Found` true)
        (break))))
  (if (not (`local.L_Found`))
    (bind _asbp_player_pawn (cast `/Game/Blueprints/Pawns/BP_PlayerPawn` (`Controller.K2_GetPawn` (`self.GetInstigatorController`))))
    (`GameplayStatics.ApplyDamage` _asbp_player_pawn 0.01))
  (`/Game/Blueprints/Enviroment/Border/BP_Border.HitProjectile` (`local.L_Border`) (`.Location` (`GameplayStatics.BreakHitResult` (`local.L_Hit`))))
  (`self.MultiDestoy`))

(fn `OnRep_Color`
  (`self.SetColorProjectile`))

(fn `OnRep_Destroyer`
  (bind _meshoverlap (`self.MeshOverlap`))
  (if (`self.Destroyer`)
    (`SceneComponent.SetHiddenInGame` _meshoverlap false false)
    (else
      (`SceneComponent.SetHiddenInGame` _meshoverlap true false))))

(fn `OnRep_Speed`
  (bind _speed (`self.Speed`))
  (set `MovementComponent.Velocity` (* (`KismetMathLibrary.MakeVector` _speed _speed _speed) (`self.GetActorForwardVector`)) (`self.ProjectileMovement`)))

(fn `SetColorProjectile`
  (bind _returnvalue (`PrimitiveComponent.CreateDynamicMaterialInstance` (`self.Mesh`) 0 "/Game/Assets/Materials/Projectile/M_Projectile_Inst.M_Projectile_Inst" "Color"))
  (bind _output_get (set `self.M_Mesh` _returnvalue))
  (`MaterialInstanceDynamic.SetVectorParameterValue` _output_get "Color" (`self.Color`)))

(fn `UserConstructionScript`)